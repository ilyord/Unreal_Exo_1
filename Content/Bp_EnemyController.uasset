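; Enemy AI controller that runs the BT_Enemy behavior tree and feeds it player perception through the Blackboard.
; Perception updates for a ThirdPersonCharacter with non-negative Health set PlayerRef when sensed.
; When sensing is lost, it stores the stimulus location as LastPlayerLocation and clears PlayerRef.
; A separate ResetPlayerRef event also clears PlayerRef.
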(event `self.AIPerception.OnTargetPerceptionUpdated`
  (params (Actor :type "Actor Object Reference") (Stimulus :type "AIStimulus Structure"))
  (bind _asthird_person_character (cast `/Game/ThirdPersonBP/Blueprints/ThirdPersonCharacter` Actor))
  (if (<= 0 (`/Game/ThirdPersonBP/Blueprints/ThirdPersonCharacter.Health` _asthird_person_character))
    (if Stimulus_bSuccessfullySensed
      (`BlackboardComponent.SetValueAsObject` (`AIBlueprintHelperLibrary.GetBlackboard` null) (`KismetStringLibrary.Conv_StringToName` "PlayerRef") _asthird_person_character)
      (else
        (`BlackboardComponent.SetValueAsVector` (`AIBlueprintHelperLibrary.GetBlackboard` null) (`KismetStringLibrary.Conv_StringToName` "LastPlayerLocation") Stimulus_StimulusLocation)
        (`BlackboardComponent.ClearValue` (`AIBlueprintHelperLibrary.GetBlackboard` null) (`KismetStringLibrary.Conv_StringToName` "PlayerRef"))))))

(event `self.ReceiveBeginPlay`
  (`self.RunBehaviorTree` "/Game/BT_Enemy.BT_Enemy"))

(event `ResetPlayerRef`
  (`BlackboardComponent.ClearValue` (`AIBlueprintHelperLibrary.GetBlackboard` null) (`KismetStringLibrary.Conv_StringToName` "PlayerRef")))

(fn `UserConstructionScript`)