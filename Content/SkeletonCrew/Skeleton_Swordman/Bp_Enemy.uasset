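; Enemy character Blueprint for a swordsman skeleton, doubling as a boss variant through IsBoss, which sets starting health and enlarges the boss.
; AnyDamage lowers Health; at zero the enemy ragdolls, loses capsule collision and detaches its controller.
; A DoOnce then adjusts the player's ThirdPersonCharacter: boss kills add health but reduce Power, while regular kills drain some health.
; Tick prints remaining life on screen as debug output.
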(event `self.ReceiveTick`
  (params (DeltaSeconds :type "Float (single-precision)"))
  (if (`self.isBoss`)
    (`KismetSystemLibrary.PrintString` (`KismetStringLibrary.Concat_StrStr` "Boss  Life " (`KismetStringLibrary.Conv_IntToString` (`self.Health`))) true true (struct :`G` 0.66 :`B` 1.0 :`A` 1.0) 0.0)
    (else
      (`KismetSystemLibrary.PrintString` (`KismetStringLibrary.Concat_StrStr` "IA Life " (`KismetStringLibrary.Conv_IntToString` (`self.Health`))) true true (struct :`G` 0.66 :`B` 1.0 :`A` 1.0) 0.0))))

(event `self.ReceiveBeginPlay`
  ;[1 1 1] Set Ennemy/Boss Life
  (if (`self.isBoss`)
    (set `self.Health` 300)
    (`self.SetActorScale3D` (2.0 2.0 2.0))
    (else
      (set `self.Health` 50))))

(event `self.ReceiveAnyDamage`
  (params (Damage :type "Float (single-precision)") (DamageType :type "DamageType Object Reference") (InstigatedBy :type "Controller Object Reference") (DamageCauser :type "Actor Object Reference"))
  (bind _output_get (set `self.Health` (`KismetMathLibrary.FTrunc` (- (`self.Health`) Damage))))
  (if (<= _output_get 0)
    (`PrimitiveComponent.SetSimulatePhysics` (`self.Mesh`) true)
    (`PrimitiveComponent.SetCollisionEnabled` (`self.CapsuleComponent`) "NoCollision")
    (`self.DetachFromControllerPendingDestroy`)
    (`SkeletalMeshComponent.SetAnimationMode` (`self.Mesh`) "AnimationSingleNode")
    (`/Engine/EditorBlueprintResources/StandardMacros.DoOnce` false
      (:`Completed`
        (bind _asthird_person_character (cast `/Game/ThirdPersonBP/Blueprints/ThirdPersonCharacter` (`GameplayStatics.GetPlayerPawn` 0)))
        ;[1 1 1] Player health and damage nerf on Boss kill
        (if (`self.isBoss`)
          (bind _health (`/Game/ThirdPersonBP/Blueprints/ThirdPersonCharacter.Health` _asthird_person_character))
          (set `/Game/ThirdPersonBP/Blueprints/ThirdPersonCharacter.Health` (+ _health 50) _asthird_person_character)
          (bind _power (`/Game/ThirdPersonBP/Blueprints/ThirdPersonCharacter.Power` _asthird_person_character))
          (if (>= _power 1)
            (set `/Game/ThirdPersonBP/Blueprints/ThirdPersonCharacter.Power` (+ _power -1) _asthird_person_character))
          (elif (>= _health 5)
            (set `/Game/ThirdPersonBP/Blueprints/ThirdPersonCharacter.Health` (- _health 5) _asthird_person_character)))))))

(fn `UserConstructionScript`)